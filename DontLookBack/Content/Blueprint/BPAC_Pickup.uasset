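; Actor component that turns its owner's static mesh into a physics pickup the first-person player can carry.
; On BeginPlay it enables physics and stores the spawn location, or destroys itself if disabled or meshless.
; Interact attaches the mesh to the player's GripPoint socket and sets the rifle animation flag; EndInteract reverses this.
; Highlighting toggles custom depth, and Respawn moves the mesh back to its spawn location when not held.
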(event `self.ReceiveBeginPlay`
  ; Setup Owner for becoming a Pickup
  (`self.IsPickupValid`
    (:`True`
      (`self.SetupPickupVars`))
    (:`False`
      (`self.K2_DestroyComponent`))))

(event `/Game/Interfaces/BPI_Interactable.Interact`
  (params (Caller :type "Actor Object Reference"))
  (bind _ownermesh (`self.OwnerMesh`))
  ; Begin Interact - Setup All
  (bind _asbp_first_person_character (cast `/Game/FirstPerson/Blueprints/BP_FirstPersonCharacter` Caller))
  (`self.SetPlayerVariables` _asbp_first_person_character)
  (`PrimitiveComponent.SetSimulatePhysics` _ownermesh false)
  (`PrimitiveComponent.SetCollisionEnabled` _ownermesh "NoCollision")
  (`SceneComponent.K2_AttachToComponent` _ownermesh (`/Game/FirstPerson/Blueprints/BP_FirstPersonCharacter.FirstPersonMesh` (`self.PlayerRef`)) "GripPoint" "SnapToTarget" "SnapToTarget" "KeepWorld" true)
  (bind _asfirst_person_anim_bp (cast `/Game/FirstPersonArms/Animations/FirstPerson_AnimBP` (`SkeletalMeshComponent.GetAnimInstance` (`/Game/FirstPerson/Blueprints/BP_FirstPersonCharacter.FirstPersonMesh` (`self.PlayerRef`)))))
  (set `/Game/FirstPersonArms/Animations/FirstPerson_AnimBP.HasRifle` true _asfirst_person_anim_bp))

(event `/Game/Interfaces/BPI_Interactable.EndInteract`
  (bind _playerref (`self.PlayerRef`))
  (bind _ownermesh (`self.OwnerMesh`))
  ; End Interact - Reset All
  (`/Engine/EditorBlueprintResources/StandardMacros.IsValid` _playerref
    (:`Is Valid`
      (set `/Game/FirstPerson/Blueprints/BP_FirstPersonCharacter.IsHoldingObject` false _playerref)
      (`PrimitiveComponent.SetCollisionEnabled` _ownermesh "QueryAndPhysics")
      (`PrimitiveComponent.SetSimulatePhysics` _ownermesh true)
      (`SceneComponent.K2_DetachFromComponent` (`self.OwnerMesh`) "KeepWorld" "KeepRelative" "KeepRelative" true)
      (bind _asfirst_person_anim_bp (cast `/Game/FirstPersonArms/Animations/FirstPerson_AnimBP` (`SkeletalMeshComponent.GetAnimInstance` (`/Game/FirstPerson/Blueprints/BP_FirstPersonCharacter.FirstPersonMesh` (`self.PlayerRef`)))))
      (set `/Game/FirstPersonArms/Animations/FirstPerson_AnimBP.HasRifle` false _asfirst_person_anim_bp)
      (`self.ResetPlayerVariables`))))

(event `/Game/Interfaces/BPI_Interactable.Highlight`
  (params (`Turn ON` :type Boolean))
  (bind _ownermesh (`self.OwnerMesh`))
  ; Highlight
  (if `Turn ON`
    (`PrimitiveComponent.SetRenderCustomDepth` _ownermesh true)
    (else
      (`PrimitiveComponent.SetRenderCustomDepth` _ownermesh false))))

(event `Respawn`
  ; Respawn
  (`/Engine/EditorBlueprintResources/StandardMacros.IsValid` (`self.PlayerRef`)
    (:`Is Not Valid`
      (`SceneComponent.K2_SetWorldLocation` (`self.OwnerMesh`) (`self.SpawnPos`) false false))))

(fn `GetHighlightColor`
  (returns (Color :type "LinearColor Structure"))
  (bind _color (`/Game/Blueprint/BPFL_GeneralStuff.GetColorFromEColor` (`self.HighlightColor`)))
  (return _color))

(fn `ResetPlayerVariables`
  (`PrimitiveComponent.SetUseCCD` (`self.OwnerMesh`) false "None")
  (set `self.PlayerRef` null)
  (set `self.PlayerCam` null))

(fn `SetPlayerVariables`
  (params (PlayerRef :type "/Game/FirstPerson/Blueprints/BP_FirstPersonCharacter Object Reference"))
  (bind _output_get (set `self.PlayerRef` PlayerRef))
  (set `/Game/FirstPerson/Blueprints/BP_FirstPersonCharacter.IsHoldingObject` true _output_get))

(fn `SetupPickupVars`
  (bind _output_get (set `self.OwnerMesh` (`Actor.GetComponentByClass` (`self.GetOwner`) "/Script/Engine.StaticMeshComponent")))
  (set `self.SpawnPos` (`SceneComponent.K2_GetComponentLocation` _output_get))
  (`PrimitiveComponent.SetCustomDepthStencilValue` _output_get 1)
  (`SceneComponent.SetMobility` _output_get "Movable")
  (`PrimitiveComponent.SetSimulatePhysics` _output_get true))